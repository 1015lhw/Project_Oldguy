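; BP_InspectComponent is a component on the first-person character that starts a camera inspection of a target actor.
; StartInspect stores the target and the owner's current camera transform, then gets the inspect transform from targets implementing BPI_Inspectable.
; It passes that transform to BP_FirstPersonCharacter and calls StartCameraInspect, leaving the camera work to the character.
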(event Custom|StartInspect
  (params (TargetActor :type Actor%20Object%20Reference))
  (Variables|Default|SetInspectTarget TargetActor)
  (Variables|Default|SetOriginalCameraTransform (Transformation|GetWorldTransform (Actor|GetComponentbyClass (Components|GetOwner) "/Script/Engine.CameraComponent")))
  (if (Utilities|DoesObjectImplementInterface (Variables|Default|GetInspectTarget) "/Game/Blueprints/BPI_Inspectable.BPI_Inspectable_C")
    (bind _transform (Class|BPIInspectable|GetInspectTransform(Message) (Variables|Default|GetInspectTarget)))
    (bind _output_get (Variables|Default|SetTargetInspectTransform _transform))
    (bind _asbp_first_person_character (Utilities|Casting|CastToBP_FirstPersonCharacter (Components|GetOwner)))
    (Variables|/Game/FirstPerson/Blueprints/BP_FirstPersonCharacter.BP_FirstPersonCharacter_C|SetTargetInspectTransform _asbp_first_person_character _output_get)
    (Default|StartCameraInspect _asbp_first_person_character)))

(event EventBeginPlay)

(event EventTick
  (params (DeltaSeconds :type Float%20%28single-precision%29)))