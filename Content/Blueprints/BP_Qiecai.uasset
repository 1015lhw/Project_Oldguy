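; BP_Qiecai is an interactable actor, apparently a vegetable-cutting station, that the player can inspect.
; On Interact it calls StartInspect on the interactor's BP_InspectComponent, then registers itself as the first-person player character's CurrentInteractingObject.
; GetInspectTransform supplies the FocusPoint component's world transform as the inspection view.
; The StartCut event is an empty stub, so no cutting logic exists here.
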(event Custom|StartCut)

(event EventBeginPlay)

(event Collision|EventActorBeginOverlap
  (params (OtherActor :type Actor%20Object%20Reference)))

(event EventTick
  (params (DeltaSeconds :type Float%20%28single-precision%29)))

(event EventInteract
  (params (Interactor :type Actor%20Object%20Reference))
  (bind _returnvalue (Actor|GetComponentbyClass Interactor "/Game/Blueprints/BP_InspectComponent.BP_InspectComponent_C"))
  (Utilities|IsValid _returnvalue
    (:Is%20Valid
      (Default|StartInspect _returnvalue self)
      (bind _asbp_first_person_character (Utilities|Casting|CastToBP_FirstPersonCharacter (Game|GetPlayerCharacter 0)))
      (Variables|/Game/FirstPerson/Blueprints/BP_FirstPersonCharacter.BP_FirstPersonCharacter_C|SetCurrentInteractingObject _asbp_first_person_character self))))

(fn ConstructionScript)

(fn GetInspectTransform
  (return (Transformation|GetWorldTransform (Variables|Default|GetFocusPoint))))