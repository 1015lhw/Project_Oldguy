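; BP_Quanjiafu is an inspectable, dust-covered prop that the player can wipe clean.
; Interact starts inspection through the interactor's BP_InspectComponent, registers the prop on the first-person character and opens the WBP_DustRag widget.
; BeginPlay gives the decal a dynamic M_Dust material, and each EraseDust call lowers its clamped opacity one step.
; GetInspectTransform returns the FocusPoint's world transform as the inspection view.
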(event Custom|EraseDust
  (bind _output_get (Variables|Default|SetCurrentDustOpacity (Math|Float|Clamp(Float) (- (Variables|Default|GetCurrentDustOpacity) 0.25))))
  (Rendering|Material|SetScalarParameterValue (Variables|Default|GetDustDecalMID) "DustOpacity" _output_get :!class /Script/Engine.MaterialInstanceDynamic))

(event EventBeginPlay
  (bind _returnvalue (Rendering|Material|CreateDynamicMaterialInstance "/Game/UIAssets/M_Dust.M_Dust" "None" "None" :!class /Script/Engine.KismetMaterialLibrary))
  (bind _output_get (Variables|Default|SetDustDecalMID _returnvalue))
  (Rendering|Components|Decal|SetDecalMaterial (Variables|Default|GetDecal) _output_get))

(event Collision|EventActorBeginOverlap
  (params (OtherActor :type Actor%20Object%20Reference)))

(event EventTick
  (params (DeltaSeconds :type Float%20%28single-precision%29)))

(event EventInteract
  (params (Interactor :type Actor%20Object%20Reference))
  (bind _returnvalue (Actor|GetComponentbyClass Interactor "/Game/Blueprints/BP_InspectComponent.BP_InspectComponent_C"))
  (Utilities|IsValid _returnvalue
    (:Is%20Valid
      (Default|StartInspect _returnvalue self)
      (bind _asbp_first_person_character (Utilities|Casting|CastToBP_FirstPersonCharacter (Game|GetPlayerCharacter 0)))
      (Variables|/Game/FirstPerson/Blueprints/BP_FirstPersonCharacter.BP_FirstPersonCharacter_C|SetCurrentInteractingObject _asbp_first_person_character self)
      (bind _returnvalue_2 (UserInterface|CreateWidget "/Game/UI/WBP_DustRag.WBP_DustRag_C"))
      (UserInterface|Viewport|AddtoViewport _returnvalue_2 0))))

(fn ConstructionScript)

(fn GetInspectTransform
  (return (Transformation|GetWorldTransform (Variables|Default|GetFocusPoint))))