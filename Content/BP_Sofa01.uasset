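; BP_Sofa01 is a sofa prop with two mesh parts whose tilt is set through rotator variables, with no active gameplay logic.
; The Construction Script takes the roll of SofaADD01 and SofaADD02, clamps each to a downward-only quarter turn (negative ninety to zero), and adds it as local rotation to its corresponding static mesh component.
; Pitch and yaw inputs are ignored.
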(event EventBeginPlay)

(event Collision|EventActorBeginOverlap
  (params (OtherActor :type Actor%20Object%20Reference)))

(event EventTick
  (params (DeltaSeconds :type Float%20%28single-precision%29)))

(fn ConstructionScript
  (Utilities|FlowControl|Sequence
    (:then_0
      (Transformation|AddLocalRotation (Variables|Default|GetStaticMeshComponent0) (Math|Rotator|MakeRotator (Math|Float|ClampAngle (.Roll (Math|Rotator|BreakRotator (Variables|Default|GetSofa_ADD_01))) -9e+01 0.0) 0.0 0.0) false false))
    (:then_1
      (Transformation|AddLocalRotation (Variables|Default|GetStaticMeshComponent02) (Math|Rotator|MakeRotator (Math|Float|ClampAngle (.Roll (Math|Rotator|BreakRotator (Variables|Default|GetSofa_ADD_02))) -9e+01 0.0) 0.0 0.0) false false))))