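; BP_WardrobeWall01 is a wall wardrobe prop whose four doors can be posed open or closed per instance.
; The construction script reads a rotator variable for each upper and lower, left and right door and adds its yaw as local rotation to that door's mesh component.
; Yaw is clamped to a quarter turn, with left and right doors swinging in opposite directions.
; The event graph has no active logic, so the doors have no runtime behavior.
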(event EventBeginPlay)

(event Collision|EventActorBeginOverlap
  (params (OtherActor :type Actor%20Object%20Reference)))

(event EventTick
  (params (DeltaSeconds :type Float%20%28single-precision%29)))

(fn ConstructionScript
  (Utilities|FlowControl|Sequence
    (:then_0
      (Transformation|AddLocalRotation (Variables|Default|GetStaticMeshComponent03) (Math|Rotator|MakeRotator 0.0 0.0 (Math|Float|ClampAngle (.Yaw (Math|Rotator|BreakRotator (Variables|Default|GetDown_Left_Door))) 0.0 9e+01)) false false))
    (:then_1
      (Transformation|AddLocalRotation (Variables|Default|GetStaticMeshComponent04) (Math|Rotator|MakeRotator 0.0 0.0 (Math|Float|ClampAngle (.Yaw (Math|Rotator|BreakRotator (Variables|Default|GetDown_Right_Door))) -9e+01 0.0)) false false))
    (:then_2
      (Transformation|AddLocalRotation (Variables|Default|GetWardrobeWall01_ADD) (Math|Rotator|MakeRotator 0.0 0.0 (Math|Float|ClampAngle (.Yaw (Math|Rotator|BreakRotator (Variables|Default|GetUp_Left_Door))) 0.0 9e+01)) false false))
    (:then_3
      (Transformation|AddLocalRotation (Variables|Default|GetStaticMeshComponent0) (Math|Rotator|MakeRotator 0.0 0.0 (Math|Float|ClampAngle (.Yaw (Math|Rotator|BreakRotator (Variables|Default|GetUp_Right_Door))) -9e+01 0.0)) false false))))